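; Base character Blueprint that supplies the animation and sound feedback for shooting, reloading and switching weapons.
; Each action event plays a montage on the Mesh, with shoot and reload choosing sounds by whether the primary weapon is equipped.
; Reload also picks a rifle or pistol montage, scaling only the rifle's play rate by ReloadTime.
; Shot sounds play at the actor's location, while reload sounds play at world origin.
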(event EventBeginPlay
  ;[0.15 0.15 0.15 0.5] Shoot
)

(event Collision|EventActorBeginOverlap
  (params (OtherActor :type Actor%20Object%20Reference))
  ;[0.15 0.15 0.15 0.5] Shoot
)

(event EventTick
  (params (DeltaSeconds :type Float%20%28single-precision%29)))

(event EventPlaySwitchWeaponAnimation
  ;[0.15 0.15 0.15 0.5] Weapon Switch
  (Animation|Montage|PlayMontage (Variables|Character|GetMesh) "/Game/Belica/Characters/Heroes/Belica/Animations/SwitchWeapon_Montage.SwitchWeapon_Montage" 3.0))

(event EventPlayShootingAnimation
  (bind _returnvalue (Transformation|GetActorLocation))
  ;[0.15 0.15 0.15 0.5] Shoot
  (Animation|Montage|PlayMontage (Variables|Character|GetMesh) "/Game/Belica/Characters/Heroes/Belica/Animations/Shoot_Montage.Shoot_Montage" 2.0
    (:then
      (if (Class|BaseCharacter|GetIsPrimaryEquipped)
        (Audio|PlaySoundatLocation "/Game/Audio/Shoot/Rifle_Shoot_Fast.Rifle_Shoot_Fast" _returnvalue "0, 0, 0" 0.1 1.0 0.0 0 0 0 0)
        (else
          (Audio|PlaySoundatLocation "/Game/Audio/Shoot/Rifle_Shoot.Rifle_Shoot" _returnvalue "0, 0, 0" 0.1 1.0 0.0 0 0 0 0))))))

(event EventPlayReloadAnimation
  (params (ReloadTime :type Float%20%28single-precision%29))
  (bind _mesh (Variables|Character|GetMesh))
  ;[0.15 0.15 0.15 0.5] Reload
  (if (Class|BaseCharacter|GetIsPrimaryEquipped)
    (Animation|Montage|PlayMontage _mesh "/Game/Belica/Characters/Heroes/Belica/Animations/WeaponAnims/Reload_Rifle.Reload_Rifle" (/ ReloadTime 3.0)
      (:then
        _))
    (else
      (Animation|Montage|PlayMontage _mesh "/Game/Belica/Characters/Heroes/Belica/Animations/WeaponAnims/Reload_Pistol_Montage.Reload_Pistol_Montage"
        (:then
          _))))
  (if (Class|BaseCharacter|GetIsPrimaryEquipped)
    (Audio|PlaySoundatLocation "/Game/Audio/Reload/Reload_Rifle.Reload_Rifle" "0, 0, 0" "0, 0, 0" 0.2 1.0 0.0 0 0 0 0)
    (else
      (Audio|PlaySoundatLocation "/Game/Audio/Reload/Reload_Pistol.Reload_Pistol" "0, 0, 0" "0, 0, 0" 0.2 1.0 0.0 0 0 0 0))))

(fn ConstructionScript)